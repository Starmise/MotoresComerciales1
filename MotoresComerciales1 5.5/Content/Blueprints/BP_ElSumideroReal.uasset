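; BP_ElSumideroReal is a spawner actor that creates a batch of BP_DummyNPC actors around itself.
; On BeginPlay it sets a five-second timer for an event that loops from zero through SumideroAmount, spawning one NPC per index.
; Each NPC lands at a random reachable navigation point near the spawner, nudged by a small offset, with yaw derived from its index and SumideroAmount.
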(event Custom|Spawn%20by%20time
  (for _index (range 0 (+ (Variables|Default|GetSumideroAmount) 0))
    (Game|SpawnActorfromClass "/Game/Blueprints/BP_DummyNPC.BP_DummyNPC_C" (Math|Transform|MakeTransform (+ (.RandomLocation (AI|Navigation|GetRandomReachablePointinRadius (Transformation|GetActorLocation) 5e+02 0 0)) (+ (Math|Vector|GetForwardVector (Math|Rotator|CombineRotators (Transformation|GetActorRotation) (Math|Rotator|MakeRotator 0.0 0.0 (Math|Conversions|ToFloat(Integer) (* _index (+ (Variables|Default|GetSumideroAmount) 300)))))) "1.000000,1.000000,1.000000")) (Math|Rotator|CombineRotators (Transformation|GetActorRotation) (Math|Rotator|MakeRotator 0.0 0.0 (Math|Conversions|ToFloat(Integer) (* _index (+ (Variables|Default|GetSumideroAmount) 300))))) "1.000000,1.000000,1.000000") "Undefined" "MultiplyWithRoot" 0 0)))

(event EventBeginPlay
  (Utilities|Time|SetTimerbyEvent (delegate Custom|Spawn%20by%20time) 5.0))

(fn ConstructionScript)