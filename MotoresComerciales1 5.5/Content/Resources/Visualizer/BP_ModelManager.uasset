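; Model manager for the visualizer that keeps a single displayed model in the level.
; On BeginPlay it spawns BP_RoboDog at a fixed transform and moves OrbCamera to a hard-coded position.
; SpawnFunctionMethod takes a class and transform, destroys any valid CurrentInstance, then spawns and stores the replacement, so it can swap models.
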(event EventBeginPlay
  (bind _output_get (Variables|Default|SetSpawnTransform (Math|Transform|MakeTransform "125.000000,0.000000,257.000000" "0, 0, 0" "1.000000,1.000000,1.000000")))
  (CallFunction|SpawnFunctionMethod "/Game/Resources/Visualizer/Models/BP_RoboDog.BP_RoboDog_C" _output_get)
  (bind _output_get_2 (Variables|Default|SetCameraSocket (Math|Transform|MakeTransform "0.000000,0.000000,240.000000" "0, 0, 0" "1.000000,1.000000,1.000000")))
  (Transformation|SetActorTransform (Variables|Default|GetOrbCamera) _output_get_2))

(fn ConstructionScript)

(fn SpawnFunctionMethod
  (params (ModelToSpawn :type Actor%20Class%20Reference) (SpawnTransform :type Transform))
  (Utilities|IsValid (Variables|Default|GetCurrentInstance)
    (:Is%20Valid
      (Actor|DestroyActor (Variables|Default|GetCurrentInstance)))
    (:Is%20Not%20Valid
      _))
  (bind _returnvalue (Game|SpawnActorfromClass ModelToSpawn SpawnTransform "Undefined" "MultiplyWithRoot" 0 0))
  (Variables|Default|SetCurrentInstance _returnvalue))