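; Orbital camera pawn for the visualizer, orbiting on a spring arm with look and zoom input.
; On BeginPlay it seeds control rotation from the camera, makes the spring arm follow it, and limits pitch between level and steeply downward.
; Look input drives controller yaw and pitch.
; Tick eases zoom input with a lerp and applies it to arm length, clamped between minimum and maximum distances.
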(event Input|EnhancedActionEvents|EnhancedInputActionIA_LookOrbital
  (params (ActionValue :type Vector%202D%20Structure) (ElapsedSeconds :type Float%20%28double-precision%29) (TriggeredSeconds :type Float%20%28double-precision%29) (InputAction :type Input%20Action%20Object%20Reference :default "/Game/Resources/Visualizer/Input/IA_LookOrbital.IA_LookOrbital"))
  (Pawn|Input|AddControllerYawInput (.x ActionValue))
  (Pawn|Input|AddControllerPitchInput (.y ActionValue)))

(event EventTick
  (params (DeltaSeconds :type Float%20%28single-precision%29))
  (bind _springarm (Variables|Default|GetSpringArm))
  ;[0.03646 0.03646 0.03646 0.5] Zoom
  (bind _output_get (Variables|Default|SetZoomDelta (Math|Float|Lerp (Variables|Default|GetZoomDelta) (Input|EnhancedActionValues|GetIA_Zoom) 0.1)))
  (Variables|/Script/Engine.SpringArmComponent|SetTargetArmLength _springarm (Math|Float|Clamp(Float) (+ (* _output_get 1.5e+02) (Variables|/Script/Engine.SpringArmComponent|GetTargetArmLength _springarm)) (Variables|Default|GetMinCameraDistance) (Variables|Default|GetMaxCameraDistance))))

(event EventBeginPlay
  (bind _returnvalue (Game|GetPlayerController 0))
  (bind _playercameramanager (Variables|/Script/Engine.PlayerController|GetPlayerCameraManager _returnvalue))
  ;[0.04896 0.04896 0.04896 0.5] Rotation
  (Pawn|SetControlRotation (Pawn|GetController) (Transformation|GetWorldRotation (Variables|Default|GetCamera)))
  (Variables|/Script/Engine.SpringArmComponent|SetbUsePawnControlRotation (Variables|Default|GetSpringArm) true)
  (Variables|/Script/Engine.PlayerCameraManager|SetViewPitchMax _playercameramanager 0.0)
  (Variables|/Script/Engine.PlayerCameraManager|SetViewPitchMin _playercameramanager -75.0))

(fn ConstructionScript)