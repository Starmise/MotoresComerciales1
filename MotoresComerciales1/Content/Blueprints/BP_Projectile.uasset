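; BP_Projectile is a projectile actor that flies forward from where it spawns and destroys itself on impact with tagged actors.
; On BeginPlay it sets the ProjectileMovement velocity along its forward vector at a fixed speed.
; Overlapping an actor tagged CollideProjectile spawns the NS_Spline_ParticleFollow Niagara effect and calls a sound spawn with no sound asset shown, then destroys the projectile.
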(event EventBeginPlay
  (Variables|/Script/Engine.MovementComponent|SetVelocity (Variables|Default|GetProjectileMovement) (* (Transformation|GetActorForwardVector) 200)))

(event Collision|EventActorBeginOverlap
  (params (OtherActor :type Actor%20Object%20Reference))
  (if (Actor|ActorHasTag OtherActor "CollideProjectile")
    (Niagara|SpawnSystematLocation "/Game/_SplineVFX/NS/NS_Spline_ParticleFollow.NS_Spline_ParticleFollow" (Transformation|GetActorLocation))
    (Audio|SpawnSoundatLocation 0 (Transformation|GetActorLocation) "0, 0, 0" 1.0 1.0 0.0 0 0)
    (Actor|DestroyActor)))

(event EventTick
  (params (DeltaSeconds :type Float%20%28single-precision%29)))

(fn ConstructionScript)